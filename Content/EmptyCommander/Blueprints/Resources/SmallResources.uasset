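; SmallResources is a resource node actor that drains itself into the game mode's CurrentResources.
; A Delay on Tick takes a fixed chunk from ResourceRemaining about once a second and prints the new total.
; ConsumeResources returns the amount taken and destroys the actor when the remainder falls short of the request.
; InitResources caches mesh boxes and fractional depletion steps, but the box-removal loop is disconnected and the steps go unused.
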(event EventTick
  (params (DeltaSeconds :type Float%20%28single-precision%29))
  (bind _gamemoderef (Variables|Default|GetGameModeRef))
  (Utilities|FlowControl|Delay 1.0)
  (if (> (Variables|Default|GetResourceRemaining) 0)
    (bind _returnedresources (CallFunction|ConsumeResources 150))
    (bind _output_get (Variables|/Game/EmptyCommander/Blueprints/GameplayBasic/Game_Mode_Base_BP.Game_Mode_Base_BP_C|SetCurrentResources _gamemoderef (+ _returnedresources (Variables|/Game/EmptyCommander/Blueprints/GameplayBasic/Game_Mode_Base_BP.Game_Mode_Base_BP_C|GetCurrentResources _gamemoderef))))
    (Development|PrintString (Utilities|String|BuildString(Integer) "Resources: " "" _output_get))))

(event EventBeginPlay
  (CallFunction|InitResources)
  (bind _asgame_mode_base_bp (Utilities|Casting|CastToGame_Mode_Base_BP (Game|GetGameMode)))
  (Variables|Default|SetGameModeRef _asgame_mode_base_bp))

(fn ConstructionScript)

(fn ConsumeResources
  (params (ResourceConsumed :type Integer))
  (if (>= (Variables|Default|GetResourceRemaining) ResourceConsumed)
    (Variables|Default|SetResourceRemaining (- (Variables|Default|GetResourceRemaining) ResourceConsumed))
    (LocalVariables|SetReturned ResourceConsumed)
    (else
      (LocalVariables|SetReturned (Variables|Default|GetResourceRemaining))
      (Variables|Default|SetResourceRemaining 0)
      (Actor|DestroyActor)))
  (return (LocalVariables|GetReturned)))

(fn InitResources
  (bind _output_get (Variables|Default|SetBoxList (Actor|GetComponentsByClass "/Script/Engine.StaticMeshComponent")))
  (Variables|Default|SetBoxCount (Utilities|Array|Length _output_get))
  (for (_ _array_index) _output_get
    (Utilities|Array|Add (Variables|Default|GetRemainingSteps) (* (Math|Conversions|ToFloat(Integer) _array_index) (/ 1.0 (Math|Conversions|ToFloat(Integer) (Utilities|Array|Length _output_get)))))))