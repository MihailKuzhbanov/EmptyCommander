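; Player controller that drives a Camera_Pawn_BP camera pawn with movement and zoom input.
; On BeginPlay it casts the player pawn and caches the reference for all input handlers.
; Move axes feed world X and Y vectors into the pawn's FloatingPawnMovement, independent of camera rotation.
; Zoom actions step the spring arm length by sensitivity times step size, checking min/max limits before each step, or reset it to default.
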(event EventBeginPlay
  (Utilities|ReferenceCast))

(event Input|ActionEvents|InputActionZoomReset
  (params (Key :type Key%20Structure))
  (:Pressed
    (Variables|/Script/Engine.SpringArmComponent|SetTargetArmLength (Variables|/Game/EmptyCommander/Blueprints/Camera_Pawn_BP.Camera_Pawn_BP_C|GetSpringArm (Variables|References|GetCamera%20Pawn%20Ref)) (Variables|ZoomValues|GetDefaultArmLength))))

(event Input|ActionEvents|InputActionZoomIn
  (params (Key :type Key%20Structure))
  (bind _camera_pawn_ref (Variables|References|GetCamera%20Pawn%20Ref))
  (bind _springarm (Variables|/Game/EmptyCommander/Blueprints/Camera_Pawn_BP.Camera_Pawn_BP_C|GetSpringArm _camera_pawn_ref))
  (:Pressed
    (if (> (Variables|/Script/Engine.SpringArmComponent|GetTargetArmLength _springarm) (Variables|ZoomValues|GetMinArmLength))
      (Variables|/Script/Engine.SpringArmComponent|SetTargetArmLength _springarm (- (Variables|/Script/Engine.SpringArmComponent|GetTargetArmLength _springarm) (* (Variables|ZoomValues|GetZoomSensetivity) (Variables|ZoomValues|GetStepArmLength)))))))

(event Input|ActionEvents|InputActionZoomOut
  (params (Key :type Key%20Structure))
  (bind _camera_pawn_ref (Variables|References|GetCamera%20Pawn%20Ref))
  (bind _springarm (Variables|/Game/EmptyCommander/Blueprints/Camera_Pawn_BP.Camera_Pawn_BP_C|GetSpringArm _camera_pawn_ref))
  (:Pressed
    (if (< (Variables|/Script/Engine.SpringArmComponent|GetTargetArmLength _springarm) (Variables|ZoomValues|GetMaxArmLength))
      (Variables|/Script/Engine.SpringArmComponent|SetTargetArmLength _springarm (+ (Variables|/Script/Engine.SpringArmComponent|GetTargetArmLength _springarm) (* (Variables|ZoomValues|GetZoomSensetivity) (Variables|ZoomValues|GetStepArmLength)))))))

(event Input|AxisEvents|InputAxisMoveForward
  (params (AxisValue :type Float%20%28single-precision%29))
  (Class|PawnMovementComponent|AddInputVector (Variables|/Game/EmptyCommander/Blueprints/Camera_Pawn_BP.Camera_Pawn_BP_C|GetFloatingPawnMovement (Variables|References|GetCamera%20Pawn%20Ref)) (Math|Vector|MakeVector AxisValue 0.0 0.0) false))

(event Input|AxisEvents|InputAxisMoveRight
  (params (AxisValue :type Float%20%28single-precision%29))
  (Class|PawnMovementComponent|AddInputVector (Variables|/Game/EmptyCommander/Blueprints/Camera_Pawn_BP.Camera_Pawn_BP_C|GetFloatingPawnMovement (Variables|References|GetCamera%20Pawn%20Ref)) (Math|Vector|MakeVector 0.0 AxisValue 0.0) false))

(fn ConstructionScript)