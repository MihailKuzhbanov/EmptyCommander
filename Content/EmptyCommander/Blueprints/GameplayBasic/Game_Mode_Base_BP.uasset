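; Base game mode Blueprint that tracks elapsed game time as hours, minutes and seconds.
; BeginPlay sets GameStarted, and Tick passes through a half-second Delay to throttle calls to ElapsedTime.
; ElapsedTime splits truncated game time into TimeStruct.
; Minutes are total minutes without wrapping at 60, and Hours divides those minutes by 3600 rather than 60.
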(event EventBeginPlay
  (Variables|Default|SetGameStarted true)
  (Variables|Default|SetTimeElapsed 0))

(event EventTick
  (params (DeltaSeconds :type Float%20%28single-precision%29))
  (Utilities|FlowControl|Delay 0.5)
  (if (Variables|Default|GetGameStarted)
    (Utilities|ElapsedTime)))

(fn ConstructionScript)