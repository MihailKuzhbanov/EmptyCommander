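; Player controller that drives a Camera_Pawn_BP with movement, zoom and yaw rotation, and owns the main HUD.
; On BeginPlay it caches pawn and GameState references, shows the mouse cursor and creates the Default_HUD widget.
; Movement axes sweep the pawn along its local axes, while zoom steps the spring arm length within limits.
; Pan inputs set a direction that Tick applies as per-frame yaw without delta-time scaling; CameraReset restores default zoom and yaw.
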(event EventBeginPlay
  (Utilities|FlowControl|Sequence
    (:then_0
      (Utilities|ReferenceCast))
    (:then_1
      (Variables|Default|SetbShowMouseCursor true))
    (:then_2
      (Utilities|SpawnWidgets)
      (UserInterface|Viewport|AddtoViewport (Variables|Default|GetGameHUDRef) 0)
      (CallFunction|SetHUDVisibility "Visible"))))

(event EventTick
  (params (DeltaSeconds :type Float%20%28single-precision%29))
  (bind _camerapawnref (Variables|Default|GetCameraPawnRef))
  (bind _returnvalue (Transformation|GetActorRotation _camerapawnref))
  (bind (_roll _pitch _yaw) (Math|Rotator|BreakRotator _returnvalue))
  (if (Variables|RotationValues|GetRotationActive)
    (Transformation|SetActorRotation _camerapawnref (Math|Rotator|MakeRotator _roll _pitch (+ _yaw (* (* (Variables|RotationValues|GetStepArmRotation) (Variables|RotationValues|GetRotationSensetivity)) (Variables|RotationValues|GetDirectionRotation)))))))

(event Input|ActionEvents|InputActionZoomIn
  (params (Key :type Key%20Structure))
  (bind _camerapawnref (Variables|Default|GetCameraPawnRef))
  (bind _springarm (Variables|/Game/EmptyCommander/Blueprints/GameplayBasic/Camera_Pawn_BP.Camera_Pawn_BP_C|GetSpringArm _camerapawnref))
  (:Pressed
    (if (> (Variables|/Script/Engine.SpringArmComponent|GetTargetArmLength _springarm) (Variables|ZoomValues|GetMinArmLength))
      (Variables|/Script/Engine.SpringArmComponent|SetTargetArmLength _springarm (- (Variables|/Script/Engine.SpringArmComponent|GetTargetArmLength _springarm) (* (Variables|ZoomValues|GetZoomSensetivity) (Variables|ZoomValues|GetStepArmLength)))))))

(event Input|ActionEvents|InputActionZoomOut
  (params (Key :type Key%20Structure))
  (bind _camerapawnref (Variables|Default|GetCameraPawnRef))
  (bind _springarm (Variables|/Game/EmptyCommander/Blueprints/GameplayBasic/Camera_Pawn_BP.Camera_Pawn_BP_C|GetSpringArm _camerapawnref))
  (:Pressed
    (if (< (Variables|/Script/Engine.SpringArmComponent|GetTargetArmLength _springarm) (Variables|ZoomValues|GetMaxArmLength))
      (Variables|/Script/Engine.SpringArmComponent|SetTargetArmLength _springarm (+ (Variables|/Script/Engine.SpringArmComponent|GetTargetArmLength _springarm) (* (Variables|ZoomValues|GetZoomSensetivity) (Variables|ZoomValues|GetStepArmLength)))))))

(event Input|ActionEvents|InputActionCameraReset
  (params (Key :type Key%20Structure))
  (bind _camerapawnref (Variables|Default|GetCameraPawnRef))
  (bind _returnvalue (Transformation|GetActorRotation _camerapawnref))
  (bind (_roll _pitch) (Math|Rotator|BreakRotator _returnvalue))
  (:Pressed
    (Variables|/Script/Engine.SpringArmComponent|SetTargetArmLength (Variables|/Game/EmptyCommander/Blueprints/GameplayBasic/Camera_Pawn_BP.Camera_Pawn_BP_C|GetSpringArm _camerapawnref) (Variables|ZoomValues|GetDefaultArmLength))
    (Transformation|SetActorRotation _camerapawnref (Math|Rotator|MakeRotator _roll _pitch (Variables|RotationValues|GetDefaultArmRotation)))))

(event Input|ActionEvents|InputActionPanLeft
  (params (Key :type Key%20Structure))
  (:Pressed
    (Variables|RotationValues|SetDirectionRotation 1.0)
    (Variables|RotationValues|SetRotationActive true))
  (:Released
    (Variables|RotationValues|SetRotationActive false)))

(event Input|ActionEvents|InputActionPanRight
  (params (Key :type Key%20Structure))
  (:Pressed
    (Variables|RotationValues|SetDirectionRotation -1.0)
    (Variables|RotationValues|SetRotationActive true))
  (:Released
    (Variables|RotationValues|SetRotationActive false)))

(event Input|AxisEvents|InputAxisMoveForward
  (params (AxisValue :type Float%20%28single-precision%29))
  (bind _camerapawnref (Variables|Default|GetCameraPawnRef))
  (bind _returnvalue (Transformation|GetActorTransform _camerapawnref))
  (Transformation|SetActorLocation _camerapawnref (+ (.Location (Math|Transform|BreakTransform _returnvalue)) (Math|Transform|TransformDirection _returnvalue (Math|Vector|MakeVector (* (* AxisValue (Variables|MovementValues|GetDefaultMovementSpeed)) (Variables|MovementValues|GetModifierMovementSpeed)) 0.0 0.0))) true false))

(event Input|AxisEvents|InputAxisMoveRight
  (params (AxisValue :type Float%20%28single-precision%29))
  (bind _camerapawnref (Variables|Default|GetCameraPawnRef))
  (bind _returnvalue (Transformation|GetActorTransform _camerapawnref))
  (Transformation|SetActorLocation _camerapawnref (+ (.Location (Math|Transform|BreakTransform _returnvalue)) (Math|Transform|TransformDirection _returnvalue (Math|Vector|MakeVector 0.0 (* (* AxisValue (Variables|MovementValues|GetDefaultMovementSpeed)) (Variables|MovementValues|GetModifierMovementSpeed)) 0.0))) true false))

(fn ConstructionScript)

(fn SetHUDVisibility
  (params (InVisibility :type ESlateVisibility%20Enum :default "Visible"))
  (Widget|SetVisibility (Variables|Default|GetGameHUDRef) InVisibility))