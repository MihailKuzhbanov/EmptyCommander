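; Player controller for an RTS that drives the camera pawn, shows the cursor and creates the HUD.
; Axis inputs move the pawn; actions zoom its spring arm, reset the view or set a yaw rotation applied on Tick.
; Select input passes tap, hold and release to the HUD, with hold timing updated only while rotation is active.
; V and C keys spawn a unit or resource at the cursor's world position.
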(event Custom|UpdateSelection
  (if (Variables|RTS|GetIsHoldingInput)
    (Variables|RTS|SetInputHoldingTime (+ (Variables|RTS|GetInputHoldingTime) (Variables|RTS|GetDeltaTime)))
    (Class|IInput|OnInputHold(Message) (Variables|Default|GetGameHUDRef))))

(event Custom|UpdateClickToMove
  (if (Variables|RTS|GetWantToMove)
    (Variables|RTS|SetMoveClickTime (+ (Variables|RTS|GetMoveClickTime) (Variables|RTS|GetDeltaTime)))))

(event EventBeginPlay
  (Utilities|FlowControl|Sequence
    (:then_0
      (Utilities|ReferenceCast))
    (:then_1
      (Variables|Default|SetbShowMouseCursor true))
    (:then_2
      (Utilities|SpawnWidgets)
      (UserInterface|Viewport|AddtoViewport (Variables|Default|GetGameHUDRef) 0)
      (CallFunction|SetHUDVisibility "Visible"))))

(event EventTick
  (params (DeltaSeconds :type Float%20%28single-precision%29))
  (bind _camerapawnref (Variables|Default|GetCameraPawnRef))
  (bind _returnvalue (Transformation|GetActorRotation _camerapawnref))
  (bind (_roll _pitch _yaw) (Math|Rotator|BreakRotator _returnvalue))
  (if (Variables|RotationValues|GetRotationActive)
    (Transformation|SetActorRotation _camerapawnref (Math|Rotator|MakeRotator _roll _pitch (+ _yaw (* (* (Variables|RotationValues|GetStepArmRotation) (Variables|RotationValues|GetRotationSensetivity)) (Variables|RotationValues|GetDirectionRotation)))))
    (CallFunction|UpdateClicktoMove)
    (CallFunction|UpdateSelection)))

(event Input|ActionEvents|InputActionSelectInput
  (params (Key :type Key%20Structure))
  (bind _gamehudref (Variables|Default|GetGameHUDRef))
  (:Pressed
    (Class|IInput|OnInputTap(Message) _gamehudref)
    (Variables|RTS|SetInputHoldingTime 0.0)
    (Variables|RTS|SetIsHoldingInput true))
  (:Released
    (Class|IInput|OnInputHoldReleased(Message) _gamehudref (Variables|RTS|GetInputHoldingTime))
    (Variables|RTS|SetIsHoldingInput true)))

(event Input|ActionEvents|InputActionZoomIn
  (params (Key :type Key%20Structure))
  (bind _camerapawnref (Variables|Default|GetCameraPawnRef))
  (bind _springarm (Variables|/Game/EmptyCommander/Blueprints/GameplayBasic/Camera_Pawn_BP.Camera_Pawn_BP_C|GetSpringArm _camerapawnref))
  (:Pressed
    (if (> (Variables|/Script/Engine.SpringArmComponent|GetTargetArmLength _springarm) (Variables|ZoomValues|GetMinArmLength))
      (Variables|/Script/Engine.SpringArmComponent|SetTargetArmLength _springarm (- (Variables|/Script/Engine.SpringArmComponent|GetTargetArmLength _springarm) (* (Variables|ZoomValues|GetZoomSensetivity) (Variables|ZoomValues|GetStepArmLength)))))))

(event Input|ActionEvents|InputActionZoomOut
  (params (Key :type Key%20Structure))
  (bind _camerapawnref (Variables|Default|GetCameraPawnRef))
  (bind _springarm (Variables|/Game/EmptyCommander/Blueprints/GameplayBasic/Camera_Pawn_BP.Camera_Pawn_BP_C|GetSpringArm _camerapawnref))
  (:Pressed
    (if (< (Variables|/Script/Engine.SpringArmComponent|GetTargetArmLength _springarm) (Variables|ZoomValues|GetMaxArmLength))
      (Variables|/Script/Engine.SpringArmComponent|SetTargetArmLength _springarm (+ (Variables|/Script/Engine.SpringArmComponent|GetTargetArmLength _springarm) (* (Variables|ZoomValues|GetZoomSensetivity) (Variables|ZoomValues|GetStepArmLength)))))))

(event Input|ActionEvents|InputActionCameraReset
  (params (Key :type Key%20Structure))
  (bind _camerapawnref (Variables|Default|GetCameraPawnRef))
  (bind _returnvalue (Transformation|GetActorRotation _camerapawnref))
  (bind (_roll _pitch) (Math|Rotator|BreakRotator _returnvalue))
  (:Pressed
    (Variables|/Script/Engine.SpringArmComponent|SetTargetArmLength (Variables|/Game/EmptyCommander/Blueprints/GameplayBasic/Camera_Pawn_BP.Camera_Pawn_BP_C|GetSpringArm _camerapawnref) (Variables|ZoomValues|GetDefaultArmLength))
    (Transformation|SetActorRotation _camerapawnref (Math|Rotator|MakeRotator _roll _pitch (Variables|RotationValues|GetDefaultArmRotation)))))

(event Input|ActionEvents|InputActionPanLeft
  (params (Key :type Key%20Structure))
  (:Pressed
    (Variables|RotationValues|SetDirectionRotation 1.0)
    (Variables|RotationValues|SetRotationActive true))
  (:Released
    (Variables|RotationValues|SetRotationActive false)))

(event Input|ActionEvents|InputActionPanRight
  (params (Key :type Key%20Structure))
  (:Pressed
    (Variables|RotationValues|SetDirectionRotation -1.0)
    (Variables|RotationValues|SetRotationActive true))
  (:Released
    (Variables|RotationValues|SetRotationActive false)))

(event Input|AxisEvents|InputAxisMoveForward
  (params (AxisValue :type Float%20%28single-precision%29))
  (bind _camerapawnref (Variables|Default|GetCameraPawnRef))
  (bind _returnvalue (Transformation|GetActorTransform _camerapawnref))
  (Transformation|SetActorLocation _camerapawnref (+ (.Location (Math|Transform|BreakTransform _returnvalue)) (Math|Transform|TransformDirection _returnvalue (Math|Vector|MakeVector (* (* AxisValue (Variables|MovementValues|GetDefaultMovementSpeed)) (Variables|MovementValues|GetModifierMovementSpeed)) 0.0 0.0))) true false))

(event Input|AxisEvents|InputAxisMoveRight
  (params (AxisValue :type Float%20%28single-precision%29))
  (bind _camerapawnref (Variables|Default|GetCameraPawnRef))
  (bind _returnvalue (Transformation|GetActorTransform _camerapawnref))
  (Transformation|SetActorLocation _camerapawnref (+ (.Location (Math|Transform|BreakTransform _returnvalue)) (Math|Transform|TransformDirection _returnvalue (Math|Vector|MakeVector 0.0 (* (* AxisValue (Variables|MovementValues|GetDefaultMovementSpeed)) (Variables|MovementValues|GetModifierMovementSpeed)) 0.0))) true false))

(event Input|KeyboardEvents|C
  (params (Key :type Key%20Structure))
  (bind _self self)
  (bind _relativecursorlocation (CallFunction|SetCursorWorldPosition _self 1e+04))
  (:Pressed
    (Game|SpawnActorfromClass "/Game/EmptyCommander/Blueprints/Resources/SmallResources.SmallResources_C" (Math|Transform|MakeTransform (Math|Vector|MakeVector (.x _relativecursorlocation) (.y _relativecursorlocation) 1.5e+02)) "Undefined" 0 0)))

(event Input|KeyboardEvents|V
  (params (Key :type Key%20Structure))
  (bind _self self)
  (bind _relativecursorlocation (CallFunction|SetCursorWorldPosition _self 1e+04))
  (:Pressed
    (Game|SpawnActorfromClass "/Game/EmptyCommander/Blueprints/Units/MasterUnit.MasterUnit_C" (Math|Transform|MakeTransform (Math|Vector|MakeVector (.x _relativecursorlocation) (.y _relativecursorlocation) 1.5e+02)) "Undefined" 0 0)))

(fn ConstructionScript)

(fn SetHUDVisibility
  (params (InVisibility :type ESlateVisibility%20Enum :default "Visible"))
  (Widget|SetVisibility (Variables|Default|GetGameHUDRef) InVisibility))

(fn SetSelectedPawns
  (params (InputSelectedPawns :type Array%20of%20Actor%20Object%20References))
  (Variables|RTS|SetSelectedPawns InputSelectedPawns))